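; Rhythm-game note actor that travels along the first lane of the level's spline actor.
; BeginPlay finds and caches the Bp_spline actor in the level.
; The move_note event plays a timeline whose track lerps distance along Lane1, setting the note's world location and rotation from the spline each update.
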(event Custom|move_note
  (bind _rhythm_spline (Variables|Default|GetRhythm_spline))
  (bind _lane1 (Variables|/Game/Characters/bp_spline.bp_spline_C|Getlane1 _rhythm_spline))
  (Components|Timeline|SetPlayRate (Variables|Default|GetTimeline) 0.1)
  (bind _newtrack_0 (Timeline|Timeline PlayFromStart)
    (:Update
      (Transformation|SetActorTransform (Math|Transform|MakeTransform (Spline|GetLocationatDistanceAlongSpline _lane1 (Math|Float|Lerp 0.0 (Spline|GetSplineLength (Variables|/Game/Characters/bp_spline.bp_spline_C|Getlane1 (Variables|Default|GetRhythm_spline))) _newtrack_0) "World") (Spline|GetRotationatDistanceAlongSpline _lane1 (Math|Float|Lerp 0.0 (Spline|GetSplineLength (Variables|/Game/Characters/bp_spline.bp_spline_C|Getlane1 (Variables|Default|GetRhythm_spline))) _newtrack_0) "World") "1.000000,1.000000,1.000000")))))

(event EventBeginPlay
  (bind _returnvalue (Actor|GetActorOfClass "/Game/Characters/bp_spline.bp_spline_C"))
  (Variables|Default|SetRhythm_spline _returnvalue))

(fn ConstructionScript)